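; VR hands Blueprint with physics-simulated hand meshes that can grab physics objects.
; On BeginPlay, physics constraints tie each simulated hand mesh, at bone hand_r for both hands, to its driving component.
; Each grab input sphere-traces forward from that hand for physics bodies and constrains a simulating hit component to the hand.
; Releasing the input breaks that hand's grab constraint.
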(event `self.ReceiveBeginPlay`
  ;[1 1 1] Physics
  (`PhysicsConstraintComponent.SetConstrainedComponents` (`self.RightPhysicsConstrant`) (`self.RightMC`) "None" (`self.RightMCMesh`) "hand_r")
  (`PrimitiveComponent.SetSimulatePhysics` (`self.RightMCMesh`) true)
  (`PrimitiveComponent.SetSimulatePhysics` (`self.LeftMCMesh`) true)
  (`PhysicsConstraintComponent.SetConstrainedComponents` (`self.LeftPhysicsConstrant`) (`self.LeftMesh`) "None" (`self.LeftMCMesh`) "hand_r"))

(event `InputAction|GrabRight`
  (params (Key :type "Key Structure"))
  (bind _rightmcmesh (`self.RightMCMesh`))
  (bind _returnvalue (`SceneComponent.K2_GetComponentLocation` _rightmcmesh))
  ;[1 1 1] Right
  (:`Pressed`
    (bind (_outhit _returnvalue_2) (`KismetSystemLibrary.SphereTraceSingleForObjects` :`Start` _returnvalue :`End` (+ (* (`KismetMathLibrary.GetForwardVector` (`SceneComponent.K2_GetComponentRotation` _rightmcmesh)) (`self.Length Of Trace`)) _returnvalue) :`Radius` 10.0 :`ObjectTypes` (`|MakeArray` "ObjectTypeQuery4" :!type "EObjectTypeQuery Enum") :`DrawDebugType` "ForOneFrame"))
    (if _returnvalue_2
      (bind (_bblockinghit _binitialoverlap _time _distance _location _impactpoint _normal _impactnormal _physmat _hitactor _hitcomponent) (`GameplayStatics.BreakHitResult` _outhit))
      (if (`SceneComponent.IsSimulatingPhysics` _hitcomponent "None")
        (`PhysicsConstraintComponent.SetConstrainedComponents` (`self.RightGrabbingConstraint`) (`self.RightMCMesh`) "None" _hitcomponent "None"))))
  (:`Released`
    (`PhysicsConstraintComponent.BreakConstraint` (`self.RightGrabbingConstraint`))))

(event `InputAction|GrabLeft`
  (params (Key :type "Key Structure"))
  (bind _leftmcmesh (`self.LeftMCMesh`))
  (bind _returnvalue (`SceneComponent.K2_GetComponentLocation` _leftmcmesh))
  ;[1 1 1] Left
  (:`Pressed`
    (bind (_outhit _returnvalue_2) (`KismetSystemLibrary.SphereTraceSingleForObjects` :`Start` _returnvalue :`End` (+ (* (`KismetMathLibrary.GetForwardVector` (`SceneComponent.K2_GetComponentRotation` _leftmcmesh)) (`self.Length Of Trace`)) _returnvalue) :`Radius` 10.0 :`ObjectTypes` (`|MakeArray` "ObjectTypeQuery4" :!type "EObjectTypeQuery Enum") :`DrawDebugType` "ForOneFrame"))
    (if _returnvalue_2
      (bind (_bblockinghit _binitialoverlap _time _distance _location _impactpoint _normal _impactnormal _physmat _hitactor _hitcomponent) (`GameplayStatics.BreakHitResult` _outhit))
      (if (`SceneComponent.IsSimulatingPhysics` _hitcomponent "None")
        (`PhysicsConstraintComponent.SetConstrainedComponents` (`self.LeftGrabbingConstraint`) (`self.LeftMCMesh`) "None" _hitcomponent "None"))))
  (:`Released`
    (`PhysicsConstraintComponent.BreakConstraint` (`self.LeftGrabbingConstraint`))))

(fn `UserConstructionScript`)